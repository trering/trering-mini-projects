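; Player character Blueprint with a power level that battery pickups recharge and the mesh material displays.
; The construction script creates a dynamic material and sets power to its initial level.
; PowerUp adds the battery's power, then a timeline lerps power from the pre-charge value to PowerLevelAfterPowerUp, which is not assigned here.
; Tick feeds the current-to-initial power ratio into the material's PowerMultiplier parameter.
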(event `self.powerUp`
  (params (batterysBatteryPower :type "Float (single-precision)"))
  (bind _powerlevel (`self.powerLevel`))
  (set `self.preChargePowerLevel` _powerlevel)
  (set `self.powerLevel` (+ batterysBatteryPower _powerlevel))
  (bind (_direction _powerupcurve) (`Timeline|PowerupTimeline` :!via `PlayFromStart`)
    (:`Update`
      (set `self.powerLevel` (`KismetMathLibrary.Lerp` (`self.preChargePowerLevel`) (`self.powerLevelAfterPowerUp`) _powerupcurve)))))

(event `self.ReceiveTick`
  (params (DeltaSeconds :type "Float (single-precision)"))
  (`parent.ReceiveTick` DeltaSeconds)
  (`MaterialInstanceDynamic.SetScalarParameterValue` (`self.Dynamic Power Material`) "PowerMultiplier" (/ (`self.powerLevel`) (`self.initialPowerLevel`))))

(fn `UserConstructionScript`
  (bind _returnvalue (`PrimitiveComponent.CreateDynamicMaterialInstance` (`self.Mesh`) 0 null))
  (set `self.Dynamic Power Material` _returnvalue)
  (set `self.powerLevel` (`self.initialPowerLevel`)))